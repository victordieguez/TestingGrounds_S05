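; Tile actor for an infinite terrain system, with a barrier that locks and unlocks as the player moves through it.
; The barrier starts solid red and turns passable green while the player overlaps LockingVolume.
; Leaving that volume relocks it and asks InfiniteTerrainGameMode_BP to spawn a tile; entering DestroyingVolume destroys this tile.
; An Arrow component supplies the attach transform through GetAttachLocation.
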(event OnComponentBeginOverlap(LockingVolume)
  (params (OverlappedComponent :type Primitive%20Component%20Object%20Reference) (OtherActor :type Actor%20Object%20Reference) (OtherComp :type Primitive%20Component%20Object%20Reference) (OtherBodyIndex :type Integer) (bFromSweep :type Boolean) (SweepResult :type Hit%20Result%20Structure%20%28by%20ref%29))
  (Utilities|IsPlayerActor OtherActor)
  (CallFunction|LockTile false))

(event OnComponentEndOverlap(LockingVolume)
  (params (OverlappedComponent :type Primitive%20Component%20Object%20Reference) (OtherActor :type Actor%20Object%20Reference) (OtherComp :type Primitive%20Component%20Object%20Reference) (OtherBodyIndex :type Integer))
  (Utilities|IsPlayerActor OtherActor)
  (CallFunction|LockTile true)
  (bind _asinfinite_terrain_game_mode_bp (Utilities|Casting|CastToInfiniteTerrainGameMode_BP (Game|GetGameMode)))
  (Default|SpawnTile _asinfinite_terrain_game_mode_bp))

(event OnComponentBeginOverlap(DestroyingVolume)
  (params (OverlappedComponent :type Primitive%20Component%20Object%20Reference) (OtherActor :type Actor%20Object%20Reference) (OtherComp :type Primitive%20Component%20Object%20Reference) (OtherBodyIndex :type Integer) (bFromSweep :type Boolean) (SweepResult :type Hit%20Result%20Structure%20%28by%20ref%29))
  (Utilities|IsPlayerActor OtherActor)
  (Actor|DestroyActor))

(event EventBeginPlay
  (CallFunction|LockTile true))

(fn ConstructionScript)

(fn GetAttachLocation
  (return (Transformation|GetWorldTransform (Variables|Default|GetArrow))))

(fn LockTile
  (params (Lock%20Tile :type Boolean))
  (bind _barrier (Variables|Default|GetBarrier))
  (Collision|SetCollisionEnabled _barrier (select Lock%20Tile "QueryAndPhysics" "NoCollision"))
  (Rendering|Material|SetMaterial _barrier 0 (select Lock%20Tile "/Game/Terrain/RedBarrier.RedBarrier" "/Game/Terrain/GreenBarrier.GreenBarrier")))